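; Game instance that acts as a shared hub for menus, saved player name, session hosting and weapon impact effects.
; Events create and remove menu, overlay and quest widgets while toggling the cursor, and store the name in a save slot.
; HostGame creates an Advanced Session with custom settings, then opens Hanamura as a listen server.
; Impact events spawn particles, with missiles adding radial damage and ultimate charge; network and travel errors are printed.
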(event Custom|Interface_Game
  (bind _returnvalue (UserInterface|CreateWidget "/Game/Interface/Overlay_game.Overlay_game_C"))
  (bind _output_get (Variables|Default|SetOverlay _returnvalue))
  (Variables|Default|SetMenu_Cross false)
  (UserInterface|Viewport|AddtoViewport _output_get 0)
  (Variables|/Script/Engine.PlayerController|SetbShowMouseCursor (Game|GetPlayerController 0) true))

(event Custom|Quest_HUD
  (bind _returnvalue (UserInterface|CreateWidget "/Game/Interface/Quest_array.Quest_array_C"))
  (bind _output_get (Variables|Default|SetQuest_UI _returnvalue))
  (Variables|Default|SetMenu_Cross false)
  (UserInterface|Viewport|AddtoViewport _output_get 0)
  (Variables|/Script/Engine.PlayerController|SetbShowMouseCursor (Game|GetPlayerController 0) true))

(event Custom|CreateMenu
  (bind _returnvalue (UserInterface|CreateWidget "/Game/Interface/Menü.Menü_C" (Game|GetPlayerController 0)))
  (Variables|Default|SetMenu _returnvalue)
  (UserInterface|Viewport|AddtoViewport (Variables|Default|GetMenu) 0)
  (Variables|/Script/Engine.PlayerController|SetbShowMouseCursor (Game|GetPlayerController 0) true)
  (Default|SoundVorher _returnvalue))

(event Custom|Set%20Normal
  (Class|BIDisplayHUD|Ammo(Message) (Variables|Default|GetDisplay_Widget) 30)
  (Variables|Default|SetHealth 200))

(event Custom|GetSavedName
  (bind _returnvalue (SaveGame|DoesSaveGameExist "SaveGame"))
  (if _returnvalue
    _))

(event Custom|Host%20Game
  (params (ServerName :type String) (Password :type String) (HasPassword :type Boolean) (GameMode :type String) (Map :type String) (MaxPlayers :type Integer))
  (|AdvancedSession (Utilities|Array|MakeArray (Class|AdvancedSessionsLibrary|MakeLiteralSessionPropertyString "ServerName" ServerName) (Class|AdvancedSessionsLibrary|MakeLiteralSessionPropertyString "Password" Password) (Class|AdvancedSessionsLibrary|MakeLiteralSessionPropertyBool "HasPassword" HasPassword) (Class|AdvancedSessionsLibrary|MakeLiteralSessionPropertyString "GameMode" GameMode) (Class|AdvancedSessionsLibrary|MakeLiteralSessionPropertyString "Map" Map)) (Game|GetPlayerController 0) MaxPlayers 0 false true false true true false false false true
    (:OnSuccess
      (Game|OpenLevel(byName) "Hanamura_Map" true "listen")
      (bind _asmy_game_instance (Utilities|Casting|CastToMyGameInstance (Game|GetGameInstance)))
      (CallFunction|WriteStates _asmy_game_instance))))

(event Custom|Quest_Remove
  (Widget|RemovefromParent (Variables|Default|GetQuest_UI))
  (Variables|Default|SetMenu_Cross true)
  (Variables|/Script/Engine.PlayerController|SetbShowMouseCursor (Game|GetPlayerController 0) false))

(event Custom|Write_States
  (bind _name (Variables|Default|GetName))
  (bind _write_players (Variables|Default|GetWrite_Players))
  (Utilities|Array|Add _write_players (Utilities|Struct|MakePlayers (.LeftS (Utilities|String|Split _name "#")) _name (Utilities|Array|Length _write_players))))

(event Custom|Interface_remove
  (Widget|RemovefromParent (Variables|Default|GetOverlay))
  (Variables|Default|SetMenu_Cross true)
  (Variables|/Script/Engine.PlayerController|SetbShowMouseCursor (Game|GetPlayerController 0) false)
  (Variables|Default|SetMenu_is_da false))

(event Custom|Destroy%20MPMenu
  (Widget|RemovefromParent (Variables|Default|GetMenu%20Widget)))

(event Custom|Hole_impact
  (params (location :type Vector) (Normal :type Vector) (Component_Attachement :type Actor%20Object%20Reference))
  (Utilities|Casting|CastToSK_Mannequin_Blueprint2 Component_Attachement
    (:CastFailed
      (Effects|SpawnEmitteratLocation "/Game/Effects/ParticleSystems/Weapons/AssaultRifle/Impacts/P_AssaultRifle_IH.P_AssaultRifle_IH" location (Math|Conversions|RotationFromXVector Normal)))))

(event Custom|SetSavedName
  (bind _returnvalue (SaveGame|DoesSaveGameExist "SaveGame"))
  (if _returnvalue
    (bind _returnvalue_2 (SaveGame|LoadGamefromSlot "SaveGame"))
    (Variables|Default|SetDave%20Game _returnvalue_2)
    (else
      (bind _returnvalue_3 (SaveGame|CreateSaveGameObject "/Game/Blueprints/DaveGame.DaveGame_C"))
      (Variables|Default|SetDave%20Game _returnvalue_3)))
  (bind _asdave_game (Utilities|Casting|CastToDaveGame (Variables|Default|GetDave%20Game)))
  (Default|ClearSave _asdave_game)
  (Variables|/Game/Blueprints/DaveGame.DaveGame_C|SetName _asdave_game (Variables|Default|GetName))
  (SaveGame|SaveGametoSlot _asdave_game "SaveGame"))

(event Custom|Missile_Impact
  (params (Location :type Vector) (Normal :type Vector) (Component%20Attachement :type Actor%20Object%20Reference))
  (Effects|SpawnEmitteratLocation "/Game/Effects/ParticleSystems/Weapons/RocketLauncher/Impact/P_Launcher_IH.P_Launcher_IH" Location (Math|Conversions|RotationFromXVector Normal))
  (bind _outactors (Actor|GetAllActorswithTag "Team2"))
  (Game|Damage|ApplyRadialDamage 1.2e+02 Location 4e+02 0 _outactors 0 0 false "ECC_Visibility")
  (bind _asfirst_person_character (Utilities|Casting|CastToFirstPersonCharacter (Game|GetPlayerCharacter 0)))
  (bind _asexp_bar_rifle (Utilities|Casting|CastToEXP_Bar_Rifle (Variables|/Game/FirstPersonBP/Blueprints/FirstPersonCharacter.FirstPersonCharacter_C|GetDisplay_Widget _asfirst_person_character)))
  (Default|FillUlti _asexp_bar_rifle 1.0))

(event Custom|CreateMPMenu
  (bind _returnvalue (UserInterface|CreateWidget "/Game/Interface/Muliplayer_Menu.Muliplayer_Menu_C" (Game|GetPlayerController 0)))
  (Variables|Default|SetMenu%20Widget _returnvalue)
  (UserInterface|Viewport|AddtoViewport (Variables|Default|GetMenu%20Widget) 0)
  (Variables|/Script/Engine.PlayerController|SetbShowMouseCursor (Game|GetPlayerController 0) true))

(event EventHandleNetworkError
  (params (FailureType :type ENetworkFailure%20Enum :default "NetDriverAlreadyExists") (bIsServer :type Boolean))
  (Development|PrintString (Utilities|String|Append (Utilities|String|Append (Utilities|String|EnumtoString FailureType) " -is Server? - ") (Utilities|String|ToString(Boolean) bIsServer)) true true "(R=0.000000,G=0.660000,B=1.000000,A=1.000000)" 2.0))

(event EventHandleTravelError
  (params (FailureType :type ETravelFailure%20Enum :default "NoLevel"))
  (Development|PrintString (Utilities|String|EnumtoString FailureType) true true "(R=0.000000,G=0.660000,B=1.000000,A=1.000000)" 2.0))

(fn OnRepReloading)